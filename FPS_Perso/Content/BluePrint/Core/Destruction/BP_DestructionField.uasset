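; BP_DestructionField is a destruction field actor that can act as a structure field, firing once enough of its supports are removed.
; On BeginPlay in structure mode, it counts the Supports array and binds RemoveAnchor to each support's RemoveFromStruct dispatcher.
; Each removal decrements SupportsAlive and calls CETrigger when the count is at or below SupportsLeftToDestroy.
; The field effect itself is not defined in these graphs.
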(event `self.ReceiveBeginPlay`
  (bind _supports (`self.Supports`))
  (`parent.ReceiveBeginPlay`)
  (if (`self.IsStructureField`)
    (set `self.SupportsAlive` (`KismetArrayLibrary.Array_Length` _supports))
    (for _array_element _supports
      (add `/Game/BluePrint/Core/Destruction/BP_Anchor.RemoveFromStruct` _array_element (delegate `RemoveAnchor`)))))

(event `RemoveAnchor`
  (bind _result (`/Engine/EditorBlueprintResources/StandardMacros.DecrementInt` (`self.SupportsAlive`))
    (:`  `
      (if (<= _result (`self.SupportsLeftToDestroy`))
        (`self.CE_Trigger`)))))

(fn `UserConstructionScript`
  (`parent.UserConstructionScript`))