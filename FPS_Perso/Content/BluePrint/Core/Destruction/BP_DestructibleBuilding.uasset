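; Destructible building actor that passes Chaos break events from its Building component on to anchor actors.
; On each break, it searches the component's InitializationFields for BP_Anchor actors and tests the break location against each anchor's BoxVolumeCol bounds.
; The first anchor containing the break has TriggerDestruction called, prints a debug string, and ends the search.
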(event `self.Building.OnChaosBreakEvent`
  (params (BreakEvent :type "ChaosBreakEvent Structure (by ref)"))
  (for _array_element (`GeometryCollectionComponent.InitializationFields` (`self.Building`))
    (bind _asbp_anchor (cast `/Game/BluePrint/Core/Destruction/BP_Anchor` _array_element))
    (bind (_origin _boxextent) (`KismetSystemLibrary.GetComponentBounds` (`/Engine/EditorResources/FieldNodes/FS_AnchorField_Generic.BoxVolumeCol` _asbp_anchor)))
    (if (`KismetMathLibrary.IsPointInBox` (`.Location` (break `ChaosBreakEvent` BreakEvent)) _origin _boxextent)
      (`|ExecutionSequence`
        (:`then_0`
          (`/Game/BluePrint/Core/Destruction/BP_Anchor.TriggerDestruction` _asbp_anchor)
          (`KismetSystemLibrary.PrintString` "Hello"))
        (:`then_1`
          (break))))))

(fn `UserConstructionScript`)