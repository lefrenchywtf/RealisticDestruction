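; Base destructible building that uses a Chaos geometry collection and field actors to drive its breakage.
; Construction registers the anchor fields under Fields as the collection's initialization fields.
; On a break event, it finds the anchor box containing the break and triggers that anchor's child master field once.
; Failing that, player-caused breaks spawn a master field at the break point, applying external strain taken from the building's damage threshold.
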(event `self.ReceiveTick`
  (params (DeltaSeconds :type "Float (single-precision)")))

(event `self.ReceiveBeginPlay`)

(event `self.Building.OnChaosBreakEvent`
  (params (BreakEvent :type "ChaosBreakEvent Structure (by ref)"))
  (for _array_element (`SceneComponent.GetChildrenComponents` (`self.Fields`) false)
    (bind _aschild_actor_component (cast `ChildActorComponent` _array_element))
    (bind _asfs_anchor_field_generic (cast `/Engine/EditorResources/FieldNodes/FS_AnchorField_Generic` (`ChildActorComponent.ChildActor` _aschild_actor_component)))
    (bind (_origin _boxextent) (`KismetSystemLibrary.GetComponentBounds` (`/Engine/EditorResources/FieldNodes/FS_AnchorField_Generic.BoxVolumeCol` _asfs_anchor_field_generic)))
    (if (`KismetMathLibrary.IsPointInBox` (`.Location` (break `ChaosBreakEvent` BreakEvent)) _origin _boxextent)
      (`|ExecutionSequence`
        (:`then_0`
          (bind _aschild_actor_component_2 (cast `ChildActorComponent` (`SceneComponent.GetChildComponent` _aschild_actor_component 1)))
          (bind _asfs_master_field (cast `/Engine/EditorResources/FieldNodes/FS_MasterField` (`ChildActorComponent.ChildActor` _aschild_actor_component_2)))
          (if (not (`/Engine/EditorResources/FieldNodes/FS_MasterField.isTriggered` _asfs_master_field))
            (`/Engine/EditorResources/FieldNodes/FS_MasterField.CE_Trigger` _asfs_master_field)
            (set `self.DestructionDone` true)
            (set `self.PlayerDestruction` false)))
        (:`then_1`
          (break)))))
  (if (and (`self.PlayerDestruction`) (not (`self.DestructionDone`)))
    (`self.Spawn Master Field External Strain` (`KismetMathLibrary.Conv_VectorToTransform` (`.Location` (break `ChaosBreakEvent` BreakEvent))) (`|GetArrayItem` (`GeometryCollectionComponent.DamageThreshold` (`self.Building`)) 1))
    (set `self.PlayerDestruction` false)
    (else
      (set `self.DestructionDone` false))))

(fn `Spawn Master Field External Strain`
  (params (SpawnTransform :type "Transform Structure") (Strain :type "Float (double-precision)"))
  (bind _returnvalue (`|SpawnActorFromClass` "/Engine/EditorResources/FieldNodes/FS_MasterField.FS_MasterField_C" SpawnTransform "Undefined" "MultiplyWithRoot" null null))
  (set `/Engine/EditorResources/FieldNodes/FS_MasterField.ActivationType` "NewEnumerator4" _returnvalue)
  (set `/Engine/EditorResources/FieldNodes/FS_MasterField.Use External Strain` true _returnvalue)
  (set `/Engine/EditorResources/FieldNodes/FS_MasterField.UseDecay` false _returnvalue)
  (set `/Engine/EditorResources/FieldNodes/FS_MasterField.UseTorque` false _returnvalue)
  (set `/Engine/EditorResources/FieldNodes/FS_MasterField.UseNoise` false _returnvalue)
  (set `/Engine/EditorResources/FieldNodes/FS_MasterField.DelayAmount` 0.0 _returnvalue)
  (set `/Engine/EditorResources/FieldNodes/FS_MasterField.Radial Magnitude` 3000.0 _returnvalue)
  (set `/Engine/EditorResources/FieldNodes/FS_MasterField.Strain Magnitude` Strain _returnvalue)
  (`/Engine/EditorResources/FieldNodes/FS_MasterField.CE_Trigger` _returnvalue))

(fn `UserConstructionScript`
  (for _array_element (`SceneComponent.GetChildrenComponents` (`self.Fields`) false)
    (bind _aschild_actor_component (cast `ChildActorComponent` _array_element))
    (bind _asfs_anchor_field_generic (cast `/Engine/EditorResources/FieldNodes/FS_AnchorField_Generic` (`ChildActorComponent.ChildActor` _aschild_actor_component)))
    (`KismetArrayLibrary.Array_Add` (`GeometryCollectionComponent.InitializationFields` (`self.Building`)) _asfs_anchor_field_generic)))