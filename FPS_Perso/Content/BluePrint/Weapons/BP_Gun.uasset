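; BP_Gun is a player weapon that provides damage and fire-animation functions for its owning BP_PlayerCharacter.
; On BeginPlay it casts its owner to that character and caches the reference.
; DoDamage applies the gun's damage to a given hit actor, and PlayGunFireAnim plays the rifle montage on the character's first-person mesh.
; Template projectile-spawn and firing-sound logic remains but is disconnected, and no hit detection happens here.
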(event `self.ReceiveBeginPlay`
  (bind _asbp_player_character (cast `/Game/BluePrint/Core/BP_PlayerCharacter` (`self.GetOwner`)))
  (set `self.First PersonCharacter` _asbp_player_character))

(fn `DoDamage`
  (params (HitActor :type "Actor Object Reference") (DamageCauser :type "Actor Object Reference"))
  (`GameplayStatics.ApplyDamage` HitActor (`self.Damage`) null DamageCauser))

(fn `PlayGunFireAnim`
  (`AnimInstance.Montage_Play` (`SkeletalMeshComponent.GetAnimInstance` (`/Game/BluePrint/Core/BP_PlayerCharacter.FirstPersonMesh` (`self.First PersonCharacter`))) "/Game/FP_Template/FirstPersonArms/Animations/FP_Rifle_Shoot_Montage.FP_Rifle_Shoot_Montage" 1.0 "MontageLength" 0.0 true))

(fn `UserConstructionScript`)