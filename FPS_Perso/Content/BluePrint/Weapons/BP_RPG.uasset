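; BP_RPG is a rocket launcher weapon Blueprint that fires physics-driven rocket projectiles.
; SpawnRocket spawns an actor of RocketClass at the given transform and copies the weapon's explosion radius and building damage onto it.
; It then launches the rocket with a mass-dependent impulse along the given direction, scaled by ProjectileVelocity.
; The event graph holds only disabled default events, and nothing in this file calls SpawnRocket.
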(fn `SpawnRocket`
  (params (SpawnPos :type "Transform Structure") (Direction :type "Vector Structure"))
  (bind _returnvalue (`|SpawnActorFromClass` (`self.RocketClass`) SpawnPos "Undefined" "MultiplyWithRoot" null null))
  (set `/Game/BluePrint/Weapons/BP_Rocket.ExplosionRadius` (`self.Projectile radius`) _returnvalue)
  (set `/Game/BluePrint/Weapons/BP_Rocket.DamageToBuilding` (`self.DamageToBuildings`) _returnvalue)
  (`PrimitiveComponent.AddImpulse` (`/Game/BluePrint/Weapons/BP_Rocket.Rocket` _returnvalue) (* (`self.ProjectileVelocity`) Direction) "None" false))

(fn `UserConstructionScript`
  (`parent.UserConstructionScript`))